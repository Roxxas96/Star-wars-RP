(event Custom|PlayerSpawnedClient
  (Utilities|HandleClientServerLogic
    (:Client
      (Utilities|IsLocalorRemote
        (:Local
          (Class|KJModPlayerProxy|SetVoiceSettings (Utilities|Struct|MakeKJModPlayerProxyVoiceSettings true true true true 3.6e+03 true 0 "" "(R=1.000000,G=1.000000,B=1.000000,A=1.000000)" "(X=0.000000,Y=0.000000)" true))
          (Class|KJModPlayerProxy|SetChatSettings (Utilities|Struct|MakeKJModPlayerProxyChatSettings true true true)))))))

(event EventInitialised
  (Utilities|HandleClientServerLogic
    (:Server
      ;[1 1 1] Server side : Update informations with local saved data
      (bind _returnvalue (Class|BlueprintJsonLibrary|LoadModiverseJSONFile "SWRP.json"))
      (if (Utilities|Enum|NotEqual(Enum) _returnvalue "")
        (if (Class|BlueprintJsonLibrary|JsonHasTypedField (Class|BlueprintJsonLibrary|ToJsonObject(String) _returnvalue) "players" "Array")
          (bind _status (Class|KJModPlayerProxy|GetPlayerStatus))
          (bind (_successful _saveplayerstruct) (CallFunction|GetLocalSavedPlayerInfo (.steamid _status) (Class|BlueprintJsonLibrary|ToArray(JsonValue) (Class|BlueprintJsonLibrary|ToJsonValue(JsonObject) (Class|BlueprintJsonLibrary|ToJsonObject(String) _returnvalue) "players"))))
          (if _successful
            (Variables|PlayerInformations|SetMoney (.Money (Utilities|Struct|BreakPlayerInformations _saveplayerstruct)))
            (Variables|PlayerInformations|SetName (.Name (Utilities|Struct|BreakPlayerInformations _saveplayerstruct)))
            (Variables|PlayerInformations|SetJob (.Job (Utilities|Struct|BreakPlayerInformations _saveplayerstruct)))
            (else
              (Variables|PlayerInformations|SetMoney 1000 :!label _label)
              (Variables|PlayerInformations|SetName (Utilities|GetDisplayName (Variables|/Script/Engine.Controller|GetPlayerState (Variables|Default|GetplayerController))))
              (Variables|PlayerInformations|SetJob "NewEnumerator0")))
          (else
            (goto _label)))
        (else
          (goto _label))))))

(event EventPlayerSpawnedwithPawn
  (Utilities|HandleClientServerLogic
    (:Server
      (Transformation|AttachActorToActor (Variables|Default|GetplayerPawn) "None" "SnapToTarget" "SnapToTarget" "SnapToTarget" true)
      (Transformation|SetActorRelativeTransform (Math|Transform|MakeTransform "0, 0, 0" "0, 0, 0" "1,1,1") false true))))

(fn ConstructionScript)

(fn OnRepName)

(fn OnRepMoney)

(fn GetLocalSavedPlayerInfo
  (params (SteamId :type String) (LocalSavedPlayersInfo :type Array%20of%20Blueprint%20Json%20Value%20Structures))
  ;[1 1 1] Get local saved informations about the player
  (bind _array_element (Utilities|Array|ForEachLoopwithBreak LocalSavedPlayersInfo :!label _label)
    (:LoopBody
      (if (Math|Boolean|ANDBoolean (Class|BlueprintJsonLibrary|JsonHasField (Class|BlueprintJsonLibrary|ToObject(JsonValue) _array_element) "steamid") (Class|BlueprintJsonLibrary|JsonHasField (Class|BlueprintJsonLibrary|ToObject(JsonValue) _array_element) "money") (Class|BlueprintJsonLibrary|JsonHasField (Class|BlueprintJsonLibrary|ToObject(JsonValue) _array_element) "name") (Class|BlueprintJsonLibrary|JsonHasField (Class|BlueprintJsonLibrary|ToObject(JsonValue) _array_element) "job"))
        (if (Utilities|Enum|Equal(Enum) SteamId (Class|BlueprintJsonLibrary|ToString(JsonValue) (Class|BlueprintJsonLibrary|ToJsonValue(JsonObject) (Class|BlueprintJsonLibrary|ToObject(JsonValue) _array_element) "steamid")))
          (LocalVariables|SetFoundPlayerInfo true)
          (LocalVariables|SetLocalSavedPlayerInfo (Utilities|Struct|MakePlayerInformations (Class|BlueprintJsonLibrary|ToString(JsonValue) (Class|BlueprintJsonLibrary|ToJsonValue(JsonObject) (Class|BlueprintJsonLibrary|ToObject(JsonValue) _array_element) "steamid")) (Class|BlueprintJsonLibrary|ToInteger(JsonValue) (Class|BlueprintJsonLibrary|ToJsonValue(JsonObject) (Class|BlueprintJsonLibrary|ToObject(JsonValue) _array_element) "money")) (Class|BlueprintJsonLibrary|ToString(JsonValue) (Class|BlueprintJsonLibrary|ToJsonValue(JsonObject) (Class|BlueprintJsonLibrary|ToObject(JsonValue) _array_element) "name")) (Utilities|Enum|ByteToEnumJobsEnum (Math|Conversions|ToByte(Integer) (Class|BlueprintJsonLibrary|ToInteger(JsonValue) (Class|BlueprintJsonLibrary|ToJsonValue(JsonObject) (Class|BlueprintJsonLibrary|ToObject(JsonValue) _array_element) "job"))))))
          (goto _label Break))))
    (:Completed
      (return (LocalVariables|GetFoundPlayerInfo) (LocalVariables|GetLocalSavedPlayerInfo)))))

(fn OnRepJob)